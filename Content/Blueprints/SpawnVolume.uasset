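; SpawnVolume is an actor that continuously spawns FloatingDebris_Child actors at random points inside its Box component.
; BeginPlay opens a gate that is never closed, so Tick feeds a 0.2-second Delay that acts as a repeating spawn timer.
; Each spawn offsets the actor's location within the scaled box extents and gets a random rotation and slightly varied, per-axis random scale.
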(event EventBeginPlay
  (bind _returnvalue (Math|Random|RandomFloatinRange 0.8 1.2))
  (bind _box (Variables|Default|GetBox))
  (bind _returnvalue_2 (Components|Box|GetScaledBoxExtent _box))
  (bind (_x _y _z) (Math|Vector|BreakVector _returnvalue_2))
  (Utilities|FlowControl|Gate true) ; enters at Open
)

(event EventActorBeginOverlap
  (params (OtherActor :type Actor%20Object%20Reference)))

(event EventTick
  (params (DeltaSeconds :type Float%20%28single-precision%29)))

(event EventTick
  (params (DeltaSeconds :type Float%20%28single-precision%29))
  (bind _returnvalue (Math|Random|RandomFloatinRange 0.8 1.2))
  (bind _box (Variables|Default|GetBox))
  (bind _returnvalue_2 (Components|Box|GetScaledBoxExtent _box))
  (bind (_x _y _z) (Math|Vector|BreakVector _returnvalue_2))
  (Utilities|FlowControl|Gate true
    (:Exit
      (Utilities|FlowControl|Delay 0.2)
      (Game|SpawnActorfromClass "/Game/Blueprints/FloatingDebris_Child.FloatingDebris_Child_C" (Math|Transform|MakeTransform (+ (Math|Vector|MakeVector (Math|Random|RandomFloatinRange (* _x -1.0) _x) (Math|Random|RandomFloatinRange (* _y -1.0) _y) (Math|Random|RandomFloatinRange (* _z -1.0) _z)) (Transformation|GetActorLocation)) (Math|Random|RandomRotator true) (Math|Vector|MakeVector _returnvalue _returnvalue _returnvalue)) "Undefined" 0 0))))

(fn ConstructionScript)