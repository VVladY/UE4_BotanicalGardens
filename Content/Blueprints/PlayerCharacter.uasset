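; Player character Blueprint that moves freely along three axes and gets pushed back by named boundary actors.
; Axis inputs add movement along the control rotation's forward, right and up vectors, while Turn and LookUp drive controller yaw and pitch.
; On overlap, it matches the other actor's object name against six side names and applies a large, fixed world-axis impulse through CharacterMovement.
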(event EventBeginPlay)

(event EventTick
  (params (DeltaSeconds :type Float%20%28single-precision%29)))

(event Collision|EventActorBeginOverlap
  (params (OtherActor :type Actor%20Object%20Reference))
  (bind _returnvalue (Utilities|GetObjectName OtherActor))
  (bind _charactermovement (Variables|Character|GetCharacterMovement))
  (if (Utilities|Enum|Equal(Enum) _returnvalue "back")
    (Physics|AddImpulse _charactermovement "200000.000000, 0, 0" false)
    (elif (Utilities|Enum|Equal(Enum) _returnvalue "front")
      (Physics|AddImpulse _charactermovement "-200000.000000, 0, 0" false)
      (elif (Utilities|Enum|Equal(Enum) _returnvalue "left")
        (Physics|AddImpulse _charactermovement "0.000000,200000.000000, 0" false)
        (elif (Utilities|Enum|Equal(Enum) _returnvalue "right")
          (Physics|AddImpulse _charactermovement "0.000000,-200000.000000, 0" false)
          (elif (Utilities|Enum|Equal(Enum) _returnvalue "top")
            (Physics|AddImpulse _charactermovement "0.000000,0.000000,-200000.000000" false)
            (elif (Utilities|Enum|Equal(Enum) _returnvalue "bottom")
              (Physics|AddImpulse _charactermovement "0.000000,0.000000,200000.000000" false))))))))

(event Input|AxisEvents|InputAxisMoveForward
  (params (AxisValue :type Float%20%28single-precision%29))
  (Pawn|Input|AddMovementInput (Math|Vector|GetForwardVector (Pawn|GetControlRotation :!class /Script/Engine.Pawn)) AxisValue false))

(event Input|AxisEvents|InputAxisMoveRight
  (params (AxisValue :type Float%20%28single-precision%29))
  (Pawn|Input|AddMovementInput (Math|Vector|GetRightVector (Pawn|GetControlRotation :!class /Script/Engine.Pawn)) AxisValue false))

(event Input|AxisEvents|InputAxisAltitude
  (params (AxisValue :type Float%20%28single-precision%29))
  (Pawn|Input|AddMovementInput (Math|Vector|GetUpVector (Pawn|GetControlRotation :!class /Script/Engine.Pawn)) AxisValue false))

(event Input|AxisEvents|InputAxisTurn
  (params (AxisValue :type Float%20%28single-precision%29))
  (Pawn|Input|AddControllerYawInput AxisValue))

(event Input|AxisEvents|InputAxisLookUp
  (params (AxisValue :type Float%20%28single-precision%29))
  (Pawn|Input|AddControllerPitchInput AxisValue))

(fn ConstructionScript)