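; Landscape Blueprint that lays a chosen mesh along a spline named ROAD, with all work done in the construction script.
; It adds one manually attached spline mesh per Spacing interval of spline length, plus one for the remainder, applying the shared material, collision toggle and forward-axis flip.
; Each segment takes world-space positions and directions at its two distances, with tangents scaled by Smoothness.
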(event EventActorBeginOverlap
  (params (OtherActor :type Actor%20Object%20Reference)))

(event EventTick
  (params (DeltaSeconds :type Float%20%28single-precision%29)))

(event EventBeginPlay)

(fn ConstructionScript
  (bind _spacing (Variables|Default|GetSpacing))
  (bind _smoothness (Variables|Default|GetSmoothness))
  (bind _road (Variables|Default|GetROAD))
  (for _index (range 0 (.ReturnValue (Math|Float|Division(WholeandRemainder) (Spline|GetSplineLength _road) _spacing)))
    (bind _returnvalue (AddComponent|AddSplineMeshComponent true))
    (Components|StaticMesh|SetStaticMesh _returnvalue (Variables|Default|GetMesh))
    (Rendering|Material|SetMaterial _returnvalue 0 (Variables|Default|GetMaterial))
    (Collision|SetCollisionEnabled _returnvalue (select (Variables|Default|GetCollision) "QueryAndPhysics" "NoCollision"))
    (SplineMesh|SetForwardAxis _returnvalue (select (Variables|Default|GetFlip%20Axis%20X/Y) "Y" "X"))
    (SplineMesh|SetStartandEnd _returnvalue (Spline|GetLocationatDistanceAlongSpline _road (* _index _spacing) "World") (* (Spline|GetDirectionatDistanceAlongSpline _road (* _index _spacing) "World") _smoothness) (Spline|GetLocationatDistanceAlongSpline _road (+ (* _index _spacing) _spacing) "World") (* (Spline|GetDirectionatDistanceAlongSpline _road (+ (* _index _spacing) _spacing) "World") _smoothness) :!class /Script/Engine.SplineMeshComponent)))